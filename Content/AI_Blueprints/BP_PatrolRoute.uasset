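; BP_PatrolRoute is an actor that supplies AI patrol locations along a spline.
; GetPatrolPointLoc steps a stored index by the current direction and returns that spline point's world location.
; The direction flips when the index reaches zero or the point count, giving a back-and-forth route.
; The route holds the index and direction itself, and its event graph and construction script are empty.
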(fn `GetPatrolPointLoc`
  (returns (PatrolLoc :type "Vector Structure"))
  (set `self.PatrolIndex` (+ (`self.PatrolIndex`) (`self.Direction`)))
  (if (or (>= (`self.PatrolIndex`) (`SplineComponent.GetNumberOfSplinePoints` (`self.Spline`))) (<= (`self.PatrolIndex`) 0))
    (set `self.Direction` (* (`self.Direction`) -1)))
  (return (`SplineComponent.GetLocationAtSplinePoint` (`self.Spline`) (`self.PatrolIndex`) "World")))

(fn `UserConstructionScript`)