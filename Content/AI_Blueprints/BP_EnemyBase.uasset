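; Base enemy character Blueprint that exposes movement, attack, aggro and patrol helpers, and handles damage and death.
; Attack plays a wheel-kick montage and signals completion even if interrupted; aggro toggles a red material and flag.
; Patrol lookup ping-pongs along a PatrolRoute spline's points, while GetIdealRange returns attack and strafe ranges.
; Point damage reduces Health, ragdolling the mesh with a radial impulse at zero or below.
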(event `Set Walk Speed`
  (params (`Max Walk Speed` :type "Float (single-precision)" :default 400.0))
  (set `CharacterMovementComponent.MaxWalkSpeed` `Max Walk Speed` (`self.CharacterMovement`)))

(event `self.ReceiveBeginPlay`
  (set `self.Original Material` (`PrimitiveComponent.GetMaterial` (`self.Mesh`) 0)))

(event `Attack`
  (`KismetSystemLibrary.PrintText` "Attack!")
  (`|PlayMontage` (`self.Mesh`) "/Game/CloseCombatAnimSet/Animations/InPlace/Attacks/NinjaWheelKick_Montage.NinjaWheelKick_Montage"
    (:`OnCompleted`
      _)
    (:`OnInterrupted`
      _))
  (`self.AttackFinished`))

(event `SetAggro`
  (`PrimitiveComponent.SetMaterial` (`self.Mesh`) 0 "/AnimationSharing/AnimSharingRed.AnimSharingRed")
  (set `self.isAggro` true))

(event `Lose Aggro`
  (`PrimitiveComponent.SetMaterial` (`self.Mesh`) 0 (`self.Original Material`))
  (set `self.isAggro` false))

(event `self.ReceivePointDamage`
  (params (Damage :type "Float (single-precision)") (DamageType :type "DamageType Object Reference") (HitLocation :type "Vector Structure") (HitNormal :type "Vector Structure") (HitComponent :type "PrimitiveComponent Object Reference") (BoneName :type Name) (ShotFromDirection :type "Vector Structure") (InstigatedBy :type "Controller Object Reference") (DamageCauser :type "Actor Object Reference") (HitInfo :type "HitResult Structure (by ref)"))
  (`KismetSystemLibrary.PrintText` (`|FormatText` "{instigator} hit me for {dmg} damage!" InstigatedBy Damage))
  (bind _output_get (set `self.Health` (- (`self.Health`) Damage)))
  (if (<= _output_get 0.0)
    (`KismetSystemLibrary.PrintString` "I am dead")
    (`self.Ragdoll` ShotFromDirection)))

(event `Ragdoll`
  (params (Origin :type "Vector Structure"))
  (`PrimitiveComponent.SetSimulatePhysics` (`self.Mesh`) true)
  (`PrimitiveComponent.AddRadialImpulse` (`self.Mesh`) (- Origin (0.0 0.0 100.0)) 300.0 25000.0 "RIF_Constant" false)
  (`CharacterMovementComponent.DisableMovement` (`self.CharacterMovement`)))

(fn `GetIdealRange`
  (returns (`Attack Range` :type "Float (double-precision)") (`Strafe Range` :type "Float (double-precision)"))
  (return (`self.Attack Range`) (`self.Strafe Range`)))

(fn `GetPatrolPointLoc`
  (returns (PatrolLoc :type "Vector Structure"))
  (set `self.PatrolIndex` (+ (`self.PatrolIndex`) (`self.Direction`)))
  (if (or (>= (`self.PatrolIndex`) (- (`SplineComponent.GetNumberOfSplinePoints` (`/Game/AI_Blueprints/BP_PatrolRoute.Spline` (`self.PatrolRoute`))) 1)) (<= (`self.PatrolIndex`) 0))
    (set `self.Direction` (* (`self.Direction`) -1)))
  (return (`SplineComponent.GetLocationAtSplinePoint` (`/Game/AI_Blueprints/BP_PatrolRoute.Spline` (`self.PatrolRoute`)) (`self.PatrolIndex`) "World")))

(fn `UserConstructionScript`)