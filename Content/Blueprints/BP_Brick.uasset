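; Throwable brick item that the player holds at the hand mesh's GunSocket and hurls as a weapon.
; Primary use locks movement during a throw montage, whose notify detaches the brick and launches it with a physics impulse, then restores walking and clears HeldItem.
; Box overlap applies point damage to BP_EnemyBase actors and reports an AI damage event.
; Secondary use is empty; an aim-montage toggle remains disconnected.
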(event `self.UseSecondary`
  (params (`Skeletal Mesh` :type "SkeletalMeshComponent Object Reference")))

(event `self.UsePrimary`
  (params (`Skeletal Mesh` :type "SkeletalMeshComponent Object Reference"))
  (if (not (`AnimInstance.Montage_IsPlaying` (`SkeletalMeshComponent.GetAnimInstance` `Skeletal Mesh`) "/Game/Blueprints/Anims/AM_ThrowBrick.AM_ThrowBrick"))
    (bind _ascharacter (cast `Character` (`ActorComponent.GetOwner` `Skeletal Mesh`)))
    (set `self.As Character` _ascharacter)
    (`CharacterMovementComponent.DisableMovement` (`Character.CharacterMovement` _ascharacter))
    (bind _notifyname (`|PlayMontage` `Skeletal Mesh` "/Game/Blueprints/Anims/AM_ThrowBrick.AM_ThrowBrick")
      (:`OnCompleted`
        (`CharacterMovementComponent.SetMovementMode` (`Character.CharacterMovement` _ascharacter) "MOVE_Walking" 0 :!label _label)
        (bind _asbp_third_person_character (cast `/Game/ThirdPerson/Blueprints/BP_ThirdPersonCharacter` _ascharacter))
        (set `/Game/ThirdPerson/Blueprints/BP_ThirdPersonCharacter.HeldItem` null _asbp_third_person_character))
      (:`OnInterrupted`
        (goto _label))
      (:`OnNotifyBegin`
        (if (== _notifyname "ThrowBrick") :!label _label_2
          (`PrimitiveComponent.SetSimulatePhysics` (`self.Brick`) true)
          (`PrimitiveComponent.SetCollisionEnabled` (`self.Box`) "QueryAndPhysics")
          (`PrimitiveComponent.SetCollisionEnabled` (`self.Brick`) "QueryAndPhysics")
          (`self.K2_DetachFromActor` "KeepWorld" "KeepWorld" "KeepWorld")
          (`PrimitiveComponent.AddImpulse` (`self.Brick`) (* (`self.GetActorForwardVector` _ascharacter) 1500.0) "None" true)))
      (:`OnNotifyEnd`
        (goto _label_2)))))

(event `self.Drop`
  (`self.K2_DetachFromActor` "KeepWorld" "KeepWorld" "KeepWorld")
  (`PrimitiveComponent.SetCollisionEnabled` (`self.Box`) "QueryAndPhysics"))

(event `self.Pickup`
  (params (SkelMesh :type "SkeletalMeshComponent Object Reference"))
  (`PrimitiveComponent.SetCollisionEnabled` (`self.Box`) "NoCollision")
  (`PrimitiveComponent.SetSimulatePhysics` (`self.Brick`) false)
  (`PrimitiveComponent.SetCollisionEnabled` (`self.Brick`) "NoCollision")
  (`SceneComponent.K2_SetWorldLocation` (`self.Brick`) (`SceneComponent.K2_GetComponentLocation` (`self.DefaultSceneRoot`)) false true)
  (`self.K2_AttachToComponent` SkelMesh "GunSocket" "SnapToTarget" "SnapToTarget" "SnapToTarget"))

(event `self.Box.OnComponentBeginOverlap`
  (params (OverlappedComponent :type "PrimitiveComponent Object Reference") (OtherActor :type "Actor Object Reference") (OtherComp :type "PrimitiveComponent Object Reference") (OtherBodyIndex :type Integer) (bFromSweep :type Boolean) (SweepResult :type "HitResult Structure (by ref)"))
  (bind (_bblockinghit _binitialoverlap _time _distance _location _impactpoint _normal _impactnormal _physmat _hitactor _hitcomponent _hitbonename _bonename _hititem _elementindex _faceindex _tracestart) (`GameplayStatics.BreakHitResult` SweepResult))
  (bind _base_damage (`self.Base Damage`))
  (bind _asbp_enemy_base (cast `/Game/AI_Blueprints/BP_EnemyBase` OtherActor))
  (`GameplayStatics.ApplyPointDamage` _asbp_enemy_base _base_damage _tracestart SweepResult (`Pawn.GetController` (`Actor.Instigator` (`Pawn.GetController` (`self.As Character`)))) self)
  (`AISense_Damage.ReportDamageEvent` _asbp_enemy_base (`GameplayStatics.GetPlayerCharacter` 0) _base_damage _tracestart))

(fn `UserConstructionScript`)