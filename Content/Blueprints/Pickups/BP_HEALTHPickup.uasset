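; Health pickup that is consumed on overlap by either the player character or a health enemy.
; For the player it applies Amount, registers itself in the save/load game mode's level stats, plays a potion sound and destroys itself.
; For the enemy it adds fixed health, sets the AI blackboard State and destroys itself.
; Its Load event swaps the cylinder to glass and halves Amount.
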(event `self.collision.OnComponentBeginOverlap`
  (params (OverlappedComponent :type "PrimitiveComponent Object Reference") (OtherActor :type "Actor Object Reference") (OtherComp :type "PrimitiveComponent Object Reference") (OtherBodyIndex :type Integer) (bFromSweep :type Boolean) (SweepResult :type "HitResult Structure (by ref)"))
  (bind _asbp_third_person_character (cast `/Game/ThirdPerson/Blueprints/BP_ThirdPersonCharacter` OtherActor)
    (:`then`
      (`/Game/ThirdPerson/Blueprints/BP_ThirdPersonCharacter.ChangeHealth` _asbp_third_person_character (`self.Amount`))
      (bind _asgm_save_load (cast `/Game/Blueprints/SaveLoad/GM_SaveLoad` (`GameplayStatics.GetGameMode`)))
      (`KismetArrayLibrary.Array_AddUnique` (`/Game/Blueprints/SaveLoad/SG_LevelStats.SaveActors` (`/Game/Blueprints/SaveLoad/GM_SaveLoad.SG_LevelStats` _asgm_save_load)) self)
      (`GameplayStatics.PlaySoundAtLocation` "/Game/Audio/172589__qubodup__health-potion-166188-drminky-potion-drink-regen.172589__qubodup__health-potion-166188-drminky-potion-drink-regen" (`self.K2_GetActorLocation`) (struct) 1.0 1.0 0.0 null null null null)
      (`self.K2_DestroyActor`))
    (:`CastFailed`
      (bind _asbp_health_enemy_child (cast `/Game/AI_Blueprints/BP_HealthEnemyChild` OtherActor))
      (set `/Game/AI_Blueprints/BP_EnemyBase.Health` (+ (`/Game/AI_Blueprints/BP_EnemyBase.Health` _asbp_health_enemy_child) 20.0) _asbp_health_enemy_child)
      (bind _output_get (set `self.aistate` "NewEnumerator0"))
      (`BlackboardComponent.SetValueAsEnum` (`AIController.Blackboard` (`/Game/AI_Blueprints/BP_EnemyBase.Health Enemy Controller` _asbp_health_enemy_child)) "State" _output_get)
      (`self.K2_DestroyActor`))))

(event `/Game/Blueprints/Interface/BPI_Savable.Load`
  (`PrimitiveComponent.SetMaterial` (`self.Cylinder`) 0 "/DatasmithContent/Materials/FBXImporter/VRED/Glass.Glass")
  (set `self.Amount` (/ (`self.Amount`) 2.0)))

(fn `UserConstructionScript`)