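; Locked door that a third-person character opens by walking into its sphere trigger while holding at least one key.
; Opening disables the trigger, spends a key, plays an unlock sound, prints the remaining count and runs a timeline lerping yaw from absolute zero to 90 degrees below the starting yaw.
; When finished, it registers itself in the game mode's level save data, and its Load event snaps the rotation open without restoring other state.
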(event `self.Sphere.OnComponentBeginOverlap`
  (params (OverlappedComponent :type "PrimitiveComponent Object Reference") (OtherActor :type "Actor Object Reference") (OtherComp :type "PrimitiveComponent Object Reference") (OtherBodyIndex :type Integer) (bFromSweep :type Boolean) (SweepResult :type "HitResult Structure (by ref)"))
  (bind _char (`self.Char`))
  (bind (_returnvalue_roll _returnvalue_pitch _returnvalue_yaw) (`KismetMathLibrary.BreakRotator` (`SceneComponent.K2_GetComponentRotation` (`self.DefaultSceneRoot`))))
  (bind (_returnvalue_roll_2 _returnvalue_pitch_2) (`KismetMathLibrary.BreakRotator` (`SceneComponent.K2_GetComponentRotation` (`self.Door`))))
  (bind _asbp_third_person_character (cast `/Game/ThirdPerson/Blueprints/BP_ThirdPersonCharacter` OtherActor))
  (bind _output_get (set `self.Char` _asbp_third_person_character))
  (if (and (> (`/Game/ThirdPerson/Blueprints/BP_ThirdPersonCharacter.KeyCount` _output_get) 0) (not (`self.bIsOpen`)))
    (`PrimitiveComponent.SetCollisionEnabled` (`self.Sphere`) "NoCollision")
    (set `self.NewDoorRotZ` (- _returnvalue_yaw 90.0))
    (set `self.bIsOpen` true)
    (bind _output_get_2 (set `/Game/ThirdPerson/Blueprints/BP_ThirdPersonCharacter.KeyCount` (- (`/Game/ThirdPerson/Blueprints/BP_ThirdPersonCharacter.KeyCount` _char) 1) _char))
    (`GameplayStatics.PlaySoundAtLocation` "/Game/Audio/519065__angelkunev__door-unlock.519065__angelkunev__door-unlock" (`self.K2_GetActorLocation`) (struct) 1.0 1.0 0.0 null null null null)
    (`KismetSystemLibrary.PrintString` (`KismetStringLibrary.Concat_StrStr` "I used a key to open a door. Total Keys Remaining: " (`KismetStringLibrary.Conv_IntToString` _output_get_2)) true true (struct :`R` 1.0 :`G` 0.398125 :`A` 1.0) 5.0)
    (bind (_direction _alpha) (`Timeline|OpenDoor` :!via `PlayFromStart`)
      (:`Update`
        (`SceneComponent.K2_SetWorldRotation` (`self.DefaultSceneRoot`) (`KismetMathLibrary.MakeRotator` _returnvalue_roll_2 _returnvalue_pitch_2 (`KismetMathLibrary.Lerp` 0.0 (`self.NewDoorRotZ`) _alpha)) false false))
      (:`Finished`
        (bind _asgm_save_load (cast `/Game/Blueprints/SaveLoad/GM_SaveLoad` (`GameplayStatics.GetGameMode`)))
        (`KismetArrayLibrary.Array_AddUnique` (`/Game/Blueprints/SaveLoad/SG_LevelStats.SaveActors` (`/Game/Blueprints/SaveLoad/GM_SaveLoad.SG_LevelStats` _asgm_save_load)) self)))))

(event `/Game/Blueprints/Interface/BPI_Savable.Load`
  (bind (_returnvalue_roll _returnvalue_pitch _returnvalue_yaw) (`KismetMathLibrary.BreakRotator` (`SceneComponent.K2_GetComponentRotation` (`self.Door`))))
  (`SceneComponent.K2_SetWorldRotation` (`self.DefaultSceneRoot`) (`KismetMathLibrary.MakeRotator` _returnvalue_roll _returnvalue_pitch (- _returnvalue_yaw 90.0)) false false))

(fn `UserConstructionScript`)