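; BP_Sword is a sword weapon that characters can pick up, drop and use.
; Pickup disables the Box collision and snaps the sword to SwordSocket on the given skeletal mesh; Drop detaches it in world space and restores collision.
; UsePrimary plays an attack montage and UseSecondary a dodge montage on the skeletal mesh passed in.
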(event `/Game/Blueprints/Interface/BPI_Item.UseSecondary`
  (params (`Skeletal Mesh` :type "SkeletalMeshComponent Object Reference"))
  (`|PlayMontage` `Skeletal Mesh` "/Game/GASMana/Animations/Attacks/AM_Dodge.AM_Dodge"))

(event `/Game/Blueprints/Interface/BPI_Item.UsePrimary`
  (params (`Skeletal Mesh` :type "SkeletalMeshComponent Object Reference"))
  (`|PlayMontage` `Skeletal Mesh` "/Game/GASMana/Animations/Attacks/AM_Attack.AM_Attack"))

(event `/Game/Blueprints/Interface/BPI_Item.Pickup`
  (params (SkelMesh :type "SkeletalMeshComponent Object Reference"))
  (`PrimitiveComponent.SetCollisionEnabled` (`self.Box`) "NoCollision")
  (`self.K2_AttachToComponent` SkelMesh "SwordSocket" "SnapToTarget" "SnapToTarget" "SnapToTarget"))

(event `/Game/Blueprints/Interface/BPI_Item.Drop`
  (`self.K2_DetachFromActor` "KeepWorld" "KeepWorld" "KeepWorld")
  (`PrimitiveComponent.SetCollisionEnabled` (`self.Box`) "QueryAndPhysics"))

(fn `UserConstructionScript`)