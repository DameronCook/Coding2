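; BP_LoopsAndLists is a demo Blueprint that prints messages to illustrate loop types and arrays.
; BeginPlay starts a self-calling Delay event, capped by DoN, which also fires an indexed for loop each pass.
; Separate events show a ForEach over colors and a counter-resetting while loop function, though nothing here calls them.
; Both for loops print indices, using color arrays to tint the text.
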(event `self.ReceiveBeginPlay`
  (`KismetSystemLibrary.PrintString` "Loops and Lists Exists")
  (`self.DelayLoop` 1.0))

(event `DelayLoop`
  (params (Duration :type "Float (single-precision)"))
  (`KismetSystemLibrary.PrintText` (`|FormatText` "This has run {count} times" (stale _counter)))
  (`KismetSystemLibrary.Delay` Duration)
  (bind _counter (`/Engine/EditorBlueprintResources/StandardMacros.Do N` 20)
    (:`Exit`
      (`self.DelayLoop` 1.0)
      (`self.Start For Loop`))))

(event `Start For Each Loop`
  (for (_array_element _array_index) (`|MakeArray` (`KismetMathLibrary.MakeColor` 0.0) (struct :`R` 1.0 :`A` 1.0) (struct :`R` 0.765207 :`B` 1.0 :`A` 1.0) (struct :`G` 1.0 :`B` 0.086951 :`A` 1.0))
    (`KismetSystemLibrary.PrintText` (`|FormatText` "This is index #{number}" _array_index) true true _array_element)))

(event `Start While Loop`
  (`self.While Loop`))

(event `Start For Loop`
  (bind _array (`|MakeArray` (`KismetMathLibrary.MakeColor` 0.0) (struct :`G` 1.0 :`B` 0.086951 :`A` 1.0) (struct :`R` 0.765207 :`B` 1.0 :`A` 1.0) (struct :`R` 1.0 :`A` 1.0) (struct :`G` 0.071334 :`B` 1.0 :`A` 1.0) (struct :`R` 1.0 :`B` 0.8424 :`A` 1.0)))
  (for _index (range (`KismetArrayLibrary.Array_Length` _array))
    (`KismetSystemLibrary.PrintText` (`|FormatText` "This is index #{number}" _index) true true (`|GetArrayItem` _array _index))))

(fn `UserConstructionScript`)

(fn `While Loop`
  (locals (Counter :type Integer :default 10))
  (while (> (`local.Counter`) 0)
    (`KismetSystemLibrary.PrintText` (`|FormatText` "There are {uses} uses in this loop" (stale _output_get)) true true (struct :`G` 1.0 :`B` 0.086951 :`A` 1.0))
    (bind _output_get (set `local.Counter` (- (`local.Counter`) 1))))
  (set `local.Counter` 10))