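; Bullet projectile that damages enemies and alerts AI, then destroys itself shortly after contact.
; Sphere hit and Sphere1 overlap run near-identical logic, applying point damage to BP_EnemyBase actors with the AsCharacter controller as instigator.
; Enemy contacts also report an AI damage-sense event crediting player 0.
; All contacts call MakeNoise, placed at the impact point for non-enemies, before a brief delay and destruction.
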(event `self.Sphere.OnComponentHit`
  (params (HitComponent :type "PrimitiveComponent Object Reference") (OtherActor :type "Actor Object Reference") (OtherComp :type "PrimitiveComponent Object Reference") (NormalImpulse :type "Vector Structure") (Hit :type "HitResult Structure (by ref)"))
  (bind (_bblockinghit _binitialoverlap _time _distance _location _impactpoint _normal _impactnormal _physmat _hitactor _hitcomponent _hitbonename _bonename _hititem _elementindex _faceindex _tracestart) (`GameplayStatics.BreakHitResult` Hit))
  (bind _base_damage (`self.Base Damage`))
  ;[1 1 1] Destroy the bullet right after it hits something.
  (bind _asbp_enemy_base (cast `/Game/AI_Blueprints/BP_EnemyBase` OtherActor)
    (:`then`
      (`GameplayStatics.ApplyPointDamage` _asbp_enemy_base _base_damage _tracestart Hit (`Pawn.GetController` (`self.As Character`)) self)
      (`AISense_Damage.ReportDamageEvent` _asbp_enemy_base (`GameplayStatics.GetPlayerCharacter` 0) _base_damage _tracestart)
      (`self.MakeNoise` 1.0 null)
      (`KismetSystemLibrary.Delay` 0.2)
      (`self.K2_DestroyActor`))
    (:`CastFailed`
      (`self.MakeNoise` 1.0 null (`.ImpactPoint` (`GameplayStatics.BreakHitResult` Hit)))
      (`KismetSystemLibrary.Delay` 0.2)
      (`self.K2_DestroyActor`))))

(event `self.Sphere1.OnComponentBeginOverlap`
  (params (OverlappedComponent :type "PrimitiveComponent Object Reference") (OtherActor :type "Actor Object Reference") (OtherComp :type "PrimitiveComponent Object Reference") (OtherBodyIndex :type Integer) (bFromSweep :type Boolean) (SweepResult :type "HitResult Structure (by ref)"))
  (bind (_bblockinghit _binitialoverlap _time _distance _location _impactpoint _normal _impactnormal _physmat _hitactor _hitcomponent _hitbonename _bonename _hititem _elementindex _faceindex _tracestart) (`GameplayStatics.BreakHitResult` SweepResult))
  (bind _base_damage (`self.Base Damage`))
  (bind _asbp_enemy_base (cast `/Game/AI_Blueprints/BP_EnemyBase` OtherActor)
    (:`then`
      (`GameplayStatics.ApplyPointDamage` _asbp_enemy_base _base_damage _tracestart SweepResult (`Pawn.GetController` (`self.As Character`)) self)
      (`AISense_Damage.ReportDamageEvent` _asbp_enemy_base (`GameplayStatics.GetPlayerCharacter` 0) _base_damage _tracestart)
      (`self.MakeNoise` 1.0 null)
      (`KismetSystemLibrary.Delay` 0.2)
      (`self.K2_DestroyActor`))
    (:`CastFailed`
      (`self.MakeNoise` 1.0 null (`.ImpactPoint` (`GameplayStatics.BreakHitResult` SweepResult)))
      (`KismetSystemLibrary.Delay` 0.5)
      (`self.K2_DestroyActor`))))

(fn `UserConstructionScript`)