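; GM_SaveLoad is a game mode that handles saving and loading player stats through the SG_PlayerStats save object in the PlayerSave slot.
; On BeginPlay it loads the slot and applies the saved Stamina to BP_ThirdPersonCharacter, or creates a new save object if none exists.
; SavePlayerStats writes the held object to disk as is, without reading the character's current Stamina, and prints the result.
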(event `self.ReceiveBeginPlay`
  (`KismetSystemLibrary.PrintString` "Loading the SaveLoadGameMode" true true (struct :`R` 1.0 :`G` 0.398125 :`A` 1.0) 10.0)
  (`self.LoadPlayerStats`))

(event `LoadPlayerStats`
  (bind _returnvalue (`GameplayStatics.DoesSaveGameExist` "PlayerSave"))
  (if _returnvalue
    (bind _returnvalue_2 (`GameplayStatics.LoadGameFromSlot` "PlayerSave"))
    (bind _assg_player_stats (cast `/Game/Blueprints/SaveLoad/SG_PlayerStats` _returnvalue_2))
    (set `self.SG_PlayerStats` _assg_player_stats)
    (bind _asbp_third_person_character (cast `/Game/ThirdPerson/Blueprints/BP_ThirdPersonCharacter` (`GameplayStatics.GetPlayerCharacter` 0)))
    (set `/Game/ThirdPerson/Blueprints/BP_ThirdPersonCharacter.Stamina` (`/Game/Blueprints/SaveLoad/SG_PlayerStats.Stamina` (`self.SG_PlayerStats`)) _asbp_third_person_character)
    (`KismetSystemLibrary.PrintString` "Player Stats have been loaded" true true (struct :`R` 1.0 :`G` 0.20883 :`A` 1.0))
    (else
      (bind _returnvalue_3 (`GameplayStatics.CreateSaveGameObject` "/Game/Blueprints/SaveLoad/SG_PlayerStats.SG_PlayerStats_C"))
      (set `self.SG_PlayerStats` _returnvalue_3))))

(event `Save Player Stats`
  (bind _returnvalue (`GameplayStatics.SaveGameToSlot` (`self.SG_PlayerStats`) "PlayerSave"))
  (if _returnvalue
    (`KismetSystemLibrary.PrintString` "Player Stats Written to file")
    (else
      (`KismetSystemLibrary.PrintString` "Player Stats not Written to file"))))

(fn `UserConstructionScript`)