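; BP_Gun is a gun that characters pick up, aim, fire and drop.
; Pickup and Drop attach it to GunSocket or detach it, toggling box collision and playing a sound.
; UseSecondary toggles aiming via AM_Aim, disabling movement; toggling off restores walking, while montage blend-out or interruption only clears the flag.
; UsePrimary, only while aiming, spawns a BP_Projectile ahead of the owner and launches it along the actor's forward vector.
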(event `/Game/Blueprints/Interface/BPI_Item.UseSecondary`
  (params (`Skeletal Mesh` :type "SkeletalMeshComponent Object Reference"))
  (if (`self.bIsAiming`)
    (set `self.bIsAiming` false)
    (bind _ascharacter (cast `Character` (`ActorComponent.GetOwner` `Skeletal Mesh`)))
    (`Character.StopAnimMontage` _ascharacter "/Game/Art/Anims/AM_Aim.AM_Aim")
    (`CharacterMovementComponent.SetMovementMode` (`Character.CharacterMovement` _ascharacter) "MOVE_Walking" 0)
    (else
      (bind _ascharacter_2 (cast `Character` (`ActorComponent.GetOwner` `Skeletal Mesh`)))
      (`|PlayMontage` `Skeletal Mesh` "/Game/Art/Anims/AM_Aim.AM_Aim"
        (:`then`
          (set `self.bIsAiming` true)
          (`CharacterMovementComponent.SetMovementMode` (`Character.CharacterMovement` _ascharacter_2) "MOVE_None" 0))
        (:`OnBlendOut`
          (set `self.bIsAiming` false :!label _label))
        (:`OnInterrupted`
          (goto _label))))))

(event `/Game/Blueprints/Interface/BPI_Item.UsePrimary`
  (params (`Skeletal Mesh` :type "SkeletalMeshComponent Object Reference"))
  (bind _returnvalue (`ActorComponent.GetOwner` `Skeletal Mesh`))
  (bind _returnvalue_2 (`self.GetActorForwardVector` _returnvalue))
  (bind _ascharacter (cast `Character` _returnvalue))
  (if (`self.bIsAiming`)
    (bind _returnvalue_3 (`|SpawnActorFromClass` "/Game/Blueprints/BP_Projectile.BP_Projectile_C" (`KismetMathLibrary.MakeTransform` (+ (`self.K2_GetActorLocation` _returnvalue) (* _returnvalue_2 100.0)) (`KismetMathLibrary.Conv_VectorToRotator` _returnvalue_2)) "Undefined" "MultiplyWithRoot" null _ascharacter null))
    (`PrimitiveComponent.SetPhysicsLinearVelocity` (`/Game/Blueprints/BP_Projectile.Sphere` _returnvalue_3) (* _returnvalue_2 10000.0) false "None")))

(event `/Game/Blueprints/Interface/BPI_Item.Drop`
  (`self.K2_DetachFromActor` "KeepWorld" "KeepWorld" "KeepWorld")
  (`PrimitiveComponent.SetCollisionEnabled` (`self.Box`) "QueryAndPhysics")
  (`GameplayStatics.PlaySoundAtLocation` "/Game/Audio/371922__mrthenoronha__single-iron-hit-hard.371922__mrthenoronha__single-iron-hit-hard" (`self.K2_GetActorLocation`) (struct) 1.0 1.0 0.0 null null null null))

(event `/Game/Blueprints/Interface/BPI_Item.Pickup`
  (params (SkelMesh :type "SkeletalMeshComponent Object Reference"))
  (`PrimitiveComponent.SetCollisionEnabled` (`self.Box`) "NoCollision")
  (`self.K2_AttachToComponent` SkelMesh "GunSocket" "SnapToTarget" "SnapToTarget" "SnapToTarget")
  (`GameplayStatics.PlaySoundAtLocation` "/Game/Audio/178186__snapper4298__camera-click_nikon.178186__snapper4298__camera-click_nikon" (`self.K2_GetActorLocation`) (struct) 1.0 1.0 0.0 null null null null))

(fn `UserConstructionScript`)