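; BP_SpawnEnemyManager populates the level with randomized AI enemies when play begins.
; It gathers every BP_EnemySpawnPoint, prints their count, and gives each a 50% chance to spawn a BP_AiMoveTo at its transform.
; Each spawned AI gets a random name, skeletal mesh and two materials by shuffling the Names, Meshes and Materials arrays and taking the first entries.
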(event `self.ReceiveBeginPlay`
  (bind _materials (`self.Materials`))
  (bind _outactors (`GameplayStatics.GetAllActorsOfClass` "/Game/Blueprints/BP_EnemySpawnPoint.BP_EnemySpawnPoint_C"))
  (`KismetSystemLibrary.PrintText` (`|FormatText` "There are {length} Spawn points in the level" (`KismetArrayLibrary.Array_Length` _outactors)))
  (for _array_element _outactors
    (if (`KismetMathLibrary.RandomBoolWithWeight` 0.5)
      (bind _returnvalue (`|SpawnActorFromClass` "/Game/AI_Blueprints/BP_AiMoveTo.BP_AiMoveTo_C" (`self.GetTransform` _array_element) "AdjustIfPossibleButAlwaysSpawn" "MultiplyWithRoot" null null))
      (`KismetArrayLibrary.Array_Shuffle` (`self.Names`))
      (`KismetArrayLibrary.Array_Shuffle` (`self.Materials`))
      (`KismetArrayLibrary.Array_Shuffle` (`self.Meshes`))
      (`TextRenderComponent.K2_SetText` (`/Game/AI_Blueprints/BP_AiMoveTo.AINameText` _returnvalue) (`|GetArrayItem` (`self.Names`)))
      (bind _mesh (`Character.Mesh` _returnvalue))
      (`PrimitiveComponent.SetMaterial` _mesh 0 (`|GetArrayItem` _materials))
      (`PrimitiveComponent.SetMaterial` _mesh 1 (`|GetArrayItem` _materials 1))
      (`SkeletalMeshComponent.SetSkeletalMeshAsset` _mesh (`|GetArrayItem` (`self.Meshes`))))))

(fn `UserConstructionScript`)